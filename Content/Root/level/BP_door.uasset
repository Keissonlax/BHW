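; BP_door is a swinging door that the player opens and closes through BP_MyChar.
; Entering the Box trigger binds the use event to the character's CollectItemDis dispatcher and sets an Overlap flag.
; Each use alternates through a FlipFlop between playing and reversing a Timeline that lerps component W's yaw.
; Leaving only clears Overlap, which use never checks, and the binding remains.
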(event `self.ReceiveBeginPlay`)

(event `use`
  (params (NewParam :type "Actor Object Reference"))
  (`/Engine/EditorBlueprintResources/StandardMacros.FlipFlop`
    (:`A`
      (bind (_direction _newtrack_0) (`Timeline|Timeline` :!label _label)
        (:`Update`
          (`SceneComponent.K2_SetRelativeRotation` (`self.w`) (`KismetMathLibrary.MakeRotator` 0.0 0.0 (`KismetMathLibrary.Lerp` 0.0 -120.0 _newtrack_0)) false false))))
    (:`B`
      (goto _label :!via `Reverse`))))

(event `self.Box.OnComponentBeginOverlap`
  (params (OverlappedComponent :type "PrimitiveComponent Object Reference") (OtherActor :type "Actor Object Reference") (OtherComp :type "PrimitiveComponent Object Reference") (OtherBodyIndex :type Integer) (bFromSweep :type Boolean) (SweepResult :type "HitResult Structure (by ref)"))
  (bind _as_bp_my_char (`self.As BP My Char`))
  (bind _asbp_my_char (cast `/Game/Root/Char/BP_MyChar` OtherActor))
  (set `self.As BP My Char` _asbp_my_char)
  (`/Engine/EditorBlueprintResources/StandardMacros.IsValid` _as_bp_my_char
    (:`Is Valid`
      (add `/Game/Root/Char/BP_MyChar.Collect Item_dis` _as_bp_my_char (delegate `use`))
      (set `self.Overlap` true))))

(event `self.Box.OnComponentEndOverlap`
  (params (OverlappedComponent :type "PrimitiveComponent Object Reference") (OtherActor :type "Actor Object Reference") (OtherComp :type "PrimitiveComponent Object Reference") (OtherBodyIndex :type Integer))
  (cast `/Game/Root/Char/BP_MyChar` OtherActor)
  (set `self.Overlap` false))

(fn `UserConstructionScript`)