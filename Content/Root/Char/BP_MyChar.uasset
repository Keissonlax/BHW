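; Player character for a cursor-aimed magic game, with input for movement, staff casting and swapping, gem collection and inventory toggling.
; BeginPlay adds the input mapping, shows the cursor and creates the main HUD.
; Tick publishes player location to a material parameter collection, yaws the capsule toward the cursor ray's ground-plane intersection, and offsets the spring arm by screen mouse position, with debug drawing.
; Mana_regen refills mana through a delayed loop.
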(event `EnhancedInput|/Game/Root/Char/iput/IA_Cast_spell`
  (params (ActionValue :type "Vector2D Structure") (ElapsedSeconds :type "Float (double-precision)") (TriggeredSeconds :type "Float (double-precision)") (InputAction :type "InputAction Object Reference" :default "/Game/Root/Char/iput/IA_Cast_spell.IA_Cast_spell"))
  (bind _bpac_staff (`self.BPAC_Staff`))
  ; Каст заклинаинй
  (:`Triggered`
    (`/Game/Root/spell/Staff/BPAC_Staff.Cast_Spell (Presed)` _bpac_staff))
  (:`Completed`
    (`/Game/Root/spell/Staff/BPAC_Staff.Cast_Spell (Relise)` _bpac_staff)))

(event `EnhancedInput|/Game/Root/Char/iput/IA_Collect_item`
  (params (ActionValue :type "Vector2D Structure") (ElapsedSeconds :type "Float (double-precision)") (TriggeredSeconds :type "Float (double-precision)") (InputAction :type "InputAction Object Reference" :default "/Game/Root/Char/iput/IA_Collect_item.IA_Collect_item"))
  ; Каст заклинаинй
  (:`Triggered`
    (message `/Game/Root/Char/I_Collect_item.Collect item` (`PrimitiveComponent.GetOverlappingActors` (`self.CapsuleComponent`) "/Game/Root/spell/SpellGem/BP_New_Magic_Gem.BP_New_Magic_Gem_C"))))

(event `EnhancedInput|/Game/Root/Char/iput/IA_Swap_staff`
  (params (ActionValue :type "Vector2D Structure") (ElapsedSeconds :type "Float (double-precision)") (TriggeredSeconds :type "Float (double-precision)") (InputAction :type "InputAction Object Reference" :default "/Game/Root/Char/iput/IA_Swap_staff.IA_Swap_staff"))
  ; Каст заклинаинй
  (:`Triggered`
    (`/Game/Root/spell/Staff/BPAC_Staff.Swap_Staff` (`self.BPAC_Staff`))))

(event `EnhancedInput|/Game/Root/Char/iput/IA_Action_BHW_Move`
  (params (ActionValue :type "Vector2D Structure") (ElapsedSeconds :type "Float (double-precision)") (TriggeredSeconds :type "Float (double-precision)") (InputAction :type "InputAction Object Reference" :default "/Game/Root/Char/iput/IA_Action_BHW_Move.IA_Action_BHW_Move"))
  (bind (_x _y) (`KismetMathLibrary.BreakVector2D` ActionValue))
  ; Comment
  (:`Triggered`
    (`self.AddMovementInput` (`KismetMathLibrary.Normal` (`KismetMathLibrary.MakeVector` _x _y)))))

(event `EnhancedInput|/Game/Root/Char/iput/IA_Action_BHW_MouseAim`
  (params (ActionValue :type "Vector2D Structure") (ElapsedSeconds :type "Float (double-precision)") (TriggeredSeconds :type "Float (double-precision)") (InputAction :type "InputAction Object Reference" :default "/Game/Root/Char/iput/IA_Action_BHW_MouseAim.IA_Action_BHW_MouseAim")))

(event `Mana_regen`
  (set `self.Can_restore_Mana?` true)
  (if (`self.Can_restore_Mana?`) :!label _label
    (set `self.Mana` (+ (`self.Mana`) 1))
    (if (>= (`self.Mana`) (`self.MAX_Mana`))
      (set `self.Can_restore_Mana?` false)
      (else
        (set `self.Can_restore_Mana?` true)
        (`KismetSystemLibrary.RetriggerableDelay` 0.1)
        (goto _label)))))

(event `self.ReceiveBeginPlay`
  (`|ExecutionSequence`
    (:`then_0`
      ; Comment
      (`|ExecutionSequence`
        (:`then_0`
          (bind _asplayer_controller (cast `PlayerController` (`self.GetController`)))
          (bind _returnvalue (pcsubsystem `EnhancedInputLocalPlayerSubsystem` _asplayer_controller))
          (`/Engine/EditorBlueprintResources/StandardMacros.IsValid` _returnvalue
            (:`Is Valid`
              (`EnhancedInputSubsystemInterface.AddMappingContext` _returnvalue "/Game/Root/Char/iput/IMC_MyGame.IMC_MyGame" 0 (struct)))))
        (:`then_1`
          (set `PlayerController.bShowMouseCursor` true (`GameplayStatics.GetPlayerController` 0)))))
    (:`then_1`
      ; Comment
      (bind _returnvalue_2 (`|CreateWidget` "/Game/Root/UI/WB_Main_UI.WB_Main_UI_C" (`GameplayStatics.GetPlayerController` 0)))
      (set `self.Main HUD` _returnvalue_2)
      (`UserWidget.AddToViewport` _returnvalue_2 0))
    (:`then_2`
      (set `self.MAX_HP` (`self.MAX_HP`))
      (set `self.MAX_Mana` (`self.Mana`)))))

(event `self.ReceiveTick`
  (params (DeltaSeconds :type "Float (single-precision)"))
  (bind (_returnvalue_x _returnvalue_y _returnvalue_z) (`KismetMathLibrary.BreakVector` (`self.K2_GetActorLocation`)))
  (`KismetMaterialLibrary.SetVectorParameterValue` "/Game/Root/Materials/OpacityShader/MPC_Player.MPC_Player" "PlayerLocation" (`KismetMathLibrary.MakeColor` _returnvalue_x _returnvalue_y _returnvalue_z))
  (`|ExecutionSequence`
    (:`then_0`
      (`self.CameraAim`))
    (:`then_1`
      (`self.test1`))
    (:`then_2`
      (bind _direction (`/Game/Root/MyFunctionLibrary.Char_vectors`))
      (`KismetSystemLibrary.PrintString` (`KismetStringLibrary.Conv_RotatorToString` (`KismetMathLibrary.Conv_VectorToRotator` _direction)) true true (struct :`R` 1.0 :`B` 0.527225 :`A` 1.0) 0.001))))

(event `CameraAim`
  (bind _returnvalue (`self.K2_GetActorLocation` self))
  (bind _location (`Controller.GetPlayerViewPoint` (`GameplayStatics.GetPlayerController` 0)))
  (bind (_bblockinghit _binitialoverlap _time _distance _location_2) (`GameplayStatics.BreakHitResult` (`PlayerController.GetHitResultUnderCursorForObjects` (`GameplayStatics.GetPlayerController` 0) (`|MakeArray` "ObjectTypeQuery1" :!type "EObjectTypeQuery Enum") true)))
  (bind (_t _intersection) (`KismetMathLibrary.LinePlaneIntersection` _location (+ (* (`KismetMathLibrary.Normal` (- (`KismetMathLibrary.MakeVector` (.x _location_2) (.y _location_2) (.z _location_2)) _location)) 5000.0) _location) (`KismetMathLibrary.MakePlaneFromPointAndNormal` (- _returnvalue (0.0 0.0 90.0)) (0.0 0.0 1.0))))
  (bind (_returnvalue_roll _returnvalue_pitch _returnvalue_yaw) (`KismetMathLibrary.BreakRotator` (`KismetMathLibrary.FindLookAtRotation` _returnvalue _intersection)))
  (`|ExecutionSequence`
    (:`then_0`
      ; смотрит в сторону курсора + дебаг
      (`SceneComponent.K2_SetWorldRotation` (`self.CapsuleComponent`) (`KismetMathLibrary.MakeRotator` 0.0 0.0 _returnvalue_yaw) false false)
      (set `self.NewVar` _returnvalue_yaw))
    (:`then_1`
      (set `self.Aim_location` _intersection)
      (`KismetSystemLibrary.DrawDebugSphere` _intersection 50.0 4 (struct :`R` 1.0 :`A` 1.0)))))

(event `EnhancedInput|/Game/Root/Char/iput/IA_Open_Inventori`
  (params (ActionValue :type "Vector2D Structure") (ElapsedSeconds :type "Float (double-precision)") (TriggeredSeconds :type "Float (double-precision)") (InputAction :type "InputAction Object Reference" :default "/Game/Root/Char/iput/IA_Open_Inventori.IA_Open_Inventori"))
  (bind _returnvalue (not (`self.Is inventori open?`)))
  ; Comment
  (:`Triggered`
    (`/Game/Root/UI/WB_Main_UI.Togle_Inventori` (`self.Main HUD`) _returnvalue)
    (set `self.Is inventori open?` _returnvalue)))

(event `test1`
  (bind (_locationx _locationy) (`PlayerController.GetMousePosition` (`GameplayStatics.GetPlayerController` 0)))
  (bind (_returnvalue_x _returnvalue_y) (`KismetMathLibrary.BreakVector2D` (* (* (- (/ (`KismetMathLibrary.MakeVector2D` _locationx _locationy) (`WidgetLayoutLibrary.GetViewportSize`)) 0.5) (1.0 -1.0)) 500.0)))
  (bind _returnvalue (+ (`KismetMathLibrary.MakeVector` (`KismetMathLibrary.SelectFloat` (* _returnvalue_y 1.5) _returnvalue_y (< _returnvalue_y 0.0)) _returnvalue_x) (`self.K2_GetActorLocation`)))
  ; Отклонение камеры
  (`KismetSystemLibrary.DrawDebugSphere` _returnvalue 10.0 4 (struct :`R` 1.0 :`G` 1.0 :`B` 1.0 :`A` 0.2))
  (`SceneComponent.K2_SetWorldLocation` (`self.SpringArm`) _returnvalue false false))

(fn `RotatePlayer`
  (bind (_returnvalue_roll _returnvalue_pitch _returnvalue_yaw) (`KismetMathLibrary.BreakRotator` (`self.K2_GetActorRotation`)))
  (bind (_returnvalue_roll_2 _returnvalue_pitch_2 _returnvalue_yaw_2) (`KismetMathLibrary.BreakRotator` (`KismetMathLibrary.RInterpTo` (`self.K2_GetActorRotation`) (`KismetMathLibrary.MakeRotator` _returnvalue_roll _returnvalue_pitch (`self.Target Rotation`)) (`GameplayStatics.GetWorldDeltaSeconds`) 10.0)))
  (if (not (`KismetMathLibrary.NearlyEqual_FloatFloat` _returnvalue_yaw (`self.Target Rotation`) 0.5))
    (`self.K2_SetActorRotation` (`KismetMathLibrary.MakeRotator` _returnvalue_roll _returnvalue_pitch _returnvalue_yaw_2))
    (return)))

(fn `SnapPlayerToFacing`
  (bind (_returnvalue_roll _returnvalue_pitch) (`KismetMathLibrary.BreakRotator` (`self.K2_GetActorRotation`)))
  (`self.K2_SetActorRotation` (`KismetMathLibrary.MakeRotator` _returnvalue_roll _returnvalue_pitch (`self.Target Rotation`)))
  (return))

(fn `UserConstructionScript`)