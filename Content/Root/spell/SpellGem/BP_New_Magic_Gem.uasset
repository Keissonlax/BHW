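; Spell gem pickup actor that gives its item to the player's inventory when collected.
; On BeginPlay it sets the crystal material according to the spell type in SpellData.
; A sphere overlap tracks whether BP_MyChar is in range, gating the CollectItem event.
; Collecting adds the item, updates the inventory slot and HUD notification, then a timeline shrinks the crystal before destroying the actor.
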(event `self.ReceiveBeginPlay`
  (bind _magiccristal (`self.MagicCristal`))
  (switch `/Game/Root/spell/E_SpellCategory` (`.Type_61_539C5CCE496AF32AC3896582DC6D72A1` (break `/Game/Root/spell/S_Spell` (`self.Spell Data`)))
    (:`NewEnumerator0`
      (`PrimitiveComponent.SetMaterial` _magiccristal 0 "/Game/Root/Char/NewMaterial1.NewMaterial1"))
    (:`NewEnumerator1`
      (`PrimitiveComponent.SetMaterial` _magiccristal 0 "/Game/Root/spell/Spell_mesh_material/NewMaterial2.NewMaterial2"))
    (:`NewEnumerator2`
      (`PrimitiveComponent.SetMaterial` _magiccristal 0 "/Game/Root/spell/Spell_mesh_material/NewMaterial1.NewMaterial1"))
    (:`NewEnumerator3`
      (`PrimitiveComponent.SetMaterial` _magiccristal 0 "/Game/Root/spell/Spell_mesh_material/NewMaterial3.NewMaterial3"))))

(event `/Game/Root/Char/I_Collect_item.Collect item`
  (bind _item_name (`self.Item Name`))
  (if (`self.Overlap`)
    (bind (_success __currentitemindex1) (`/Game/Root/spell/Inventory/BPAC_New_Inventory.Add_Item` (`/Game/Root/Char/BP_MyChar.BPAC_New_Inventory` (stale `self.Sphere.OnComponentBeginOverlap` _asbp_my_char)) (`self.Item Name`) 0))
    (bind _main_hud (`/Game/Root/Char/BP_MyChar.Main HUD` (stale `self.Sphere.OnComponentBeginOverlap` _asbp_my_char)))
    (`/Game/Root/UI/WB_New_Inventory_Slot.Update_slot` (`|GetArrayItem` (`/Game/Root/UI/WB_Base_Inventory_UI.Base_Inventory_Slots` (`/Game/Root/UI/WB_Main_UI.WB_Base_Inventory_UI` _main_hud)) __currentitemindex1) _item_name)
    (`/Game/Root/UI/WB_Notification_UI.Init_Notification` (`/Game/Root/UI/WB_Main_UI.WB_Notification_UI` _main_hud) _item_name)
    (`/Game/Root/UI/WB_Main_UI.Collect_Item_anim` _main_hud)
    (bind (_direction _newtrack_0) (`Timeline|Timeline`)
      (:`Update`
        (`SceneComponent.SetRelativeScale3D` (`self.MagicCristal`) (`KismetMathLibrary.Conv_DoubleToVector` (`KismetMathLibrary.Lerp` 1.0 0.0 _newtrack_0))))
      (:`Finished`
        (`self.K2_DestroyActor`)))))

(event `self.Sphere.OnComponentBeginOverlap`
  (params (OverlappedComponent :type "PrimitiveComponent Object Reference") (OtherActor :type "Actor Object Reference") (OtherComp :type "PrimitiveComponent Object Reference") (OtherBodyIndex :type Integer) (bFromSweep :type Boolean) (SweepResult :type "HitResult Structure (by ref)"))
  (bind _asbp_my_char (cast `/Game/Root/Char/BP_MyChar` OtherActor))
  (set `self.Overlap` true))

(event `self.Sphere.OnComponentEndOverlap`
  (params (OverlappedComponent :type "PrimitiveComponent Object Reference") (OtherActor :type "Actor Object Reference") (OtherComp :type "PrimitiveComponent Object Reference") (OtherBodyIndex :type Integer))
  (cast `/Game/Root/Char/BP_MyChar` OtherActor)
  (set `self.Overlap` false))

(fn `UserConstructionScript`)