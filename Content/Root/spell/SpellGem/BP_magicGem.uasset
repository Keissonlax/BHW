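; BP_magicGem is a spell gem world pickup that loads its spell data from DT_Spell by SpellID on BeginPlay.
; A sphere overlap with BP_MyChar caches the character and sets an Overlap flag.
; Logic to add the item to inventory, show a HUD notification and destroy the gem exists but is unconnected, as is a crystal bobbing timeline.
; The CollectItem event is empty.
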(event `self.ReceiveBeginPlay`
  (`self.Data set`))

(event `/Game/Root/Char/I_Collect_item.Collect item`)

(event `self.Sphere.OnComponentBeginOverlap`
  (params (OverlappedComponent :type "PrimitiveComponent Object Reference") (OtherActor :type "Actor Object Reference") (OtherComp :type "PrimitiveComponent Object Reference") (OtherBodyIndex :type Integer) (bFromSweep :type Boolean) (SweepResult :type "HitResult Structure (by ref)"))
  (bind _asbp_my_char (cast `/Game/Root/Char/BP_MyChar` OtherActor))
  (set `self.Overlap` true))

(event `self.Sphere.OnComponentEndOverlap`
  (params (OverlappedComponent :type "PrimitiveComponent Object Reference") (OtherActor :type "Actor Object Reference") (OtherComp :type "PrimitiveComponent Object Reference") (OtherBodyIndex :type Integer))
  (set `self.Overlap` false))

(fn `Data set`
  (bind _returnvalue (`|GetDataTableRow` "/Game/Root/spell/DT_Spell.DT_Spell" (`KismetStringLibrary.Conv_StringToName` (`self.Spell ID`)))
    (:`then`
      (set `self.Spell Data` _returnvalue))))

(fn `UserConstructionScript`)