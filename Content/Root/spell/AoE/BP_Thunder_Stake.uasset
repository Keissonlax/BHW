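; Thunder Stake AoE spell actor that moves its root to the player character's AimLocation on BeginPlay.
; A collapsed graph creates a dynamic material for MagicBall, then sets its opacity, its scale and the Lightning component's height from Timeline tracks, with Lerps for scale and height.
; Nothing starts the Timeline, so these values apply only once rather than animating the ball and descending bolt.
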(event EventBeginPlay
  (|CallParentFunction)
  (bind _asbp_my_char (Utilities|Casting|CastToBP_MyChar (Game|Player|GetPlayerPawn 0)))
  (Transformation|SetWorldLocation (Variables|Default|GetDefaultSceneRoot) (Variables|/Game/Root/Char/BP_MyChar.BP_MyChar_C|GetAim_location _asbp_my_char) false false)
  (|CollapseGraph))

(event Collision|EventActorBeginOverlap
  (params (OtherActor :type Actor%20Object%20Reference))
  (|CallParentFunction OtherActor) ; This node is disabled and will not be called.\nDrag off pins to build functionality.
)

(event EventTick
  (params (DeltaSeconds :type Float%20%28single-precision%29))
  (|CallParentFunction DeltaSeconds) ; This node is disabled and will not be called.\nDrag off pins to build functionality.
)

(fn ConstructionScript
  (|CallParentFunction))