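; Thorn bush area-of-effect spell actor that grows a ring of meshes around its origin.
; The construction script spaces offsets by yaw at a fixed radius from the root's forward vector, previewing them with debug spheres.
; BeginPlay snaps the root to the character's aim height, adds a mesh and collision sphere at each offset, then scales the meshes up via a timeline.
; No overlap effect is implemented.
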(event `self.ReceiveBeginPlay`
  (bind _defaultsceneroot (`self.DefaultSceneRoot`))
  (bind (_returnvalue_x _returnvalue_y) (`KismetMathLibrary.BreakVector` (`SceneComponent.K2_GetComponentLocation` _defaultsceneroot)))
  (bind (_aim_location_x _aim_location_y _aim_location_z) (`KismetMathLibrary.BreakVector` (`/Game/Root/Char/BP_MyChar.Aim_location` (`self.As BP My Char`))))
  (`parent.ReceiveBeginPlay`)
  (`SceneComponent.K2_SetWorldLocation` _defaultsceneroot (`KismetMathLibrary.MakeVector` _returnvalue_x _returnvalue_y _aim_location_z) false false)
  (for _array_element (`self.NewVar_0`)
    (bind _returnvalue (`AddComponent|NODE_AddStaticMeshComponent-0` :`RelativeTransform` (`KismetMathLibrary.MakeTransform` _array_element)))
    (`KismetArrayLibrary.Array_Add` (`self.Static Mesh`) _returnvalue)
    (bind _returnvalue_2 (`AddComponent|NODE_AddSphereComponent-0` :`RelativeTransform` (`KismetMathLibrary.MakeTransform` _array_element)))
    (`KismetArrayLibrary.Array_Add` (`self.Spere Collision`) _returnvalue_2))
  (bind (_direction _newtrack_0) (`Timeline|Timeline`)
    (:`Update`
      (for _array_element_2 (`self.Static Mesh`)
        (`SceneComponent.SetRelativeScale3D` _array_element_2 (`KismetMathLibrary.Conv_DoubleToVector` (`KismetMathLibrary.Lerp` 0.0 1.0 _newtrack_0)))))))

(event `self.ReceiveTick`
  (params (DeltaSeconds :type "Float (single-precision)"))
  (`parent.ReceiveTick` DeltaSeconds))

(fn `UserConstructionScript`
  (locals (NewLocalVar :type Integer :default 5) (NewLocalVar_0 :type "Float (double-precision)" :default 360.0) (NewLocalVar_1 :type "Array of Vector Structure"))
  (`parent.UserConstructionScript`)
  (for _index (range (`local.NewLocalVar`))
    (bind _returnvalue (`KismetMathLibrary.GreaterGreater_VectorRotator` (* (`KismetMathLibrary.Normal` (`SceneComponent.GetForwardVector` (`self.DefaultSceneRoot`))) 200.0) (`KismetMathLibrary.MakeRotator` 0.0 0.0 (* (+ _index 1) (/ (`local.NewLocalVar_0`) (`local.NewLocalVar`))))))
    (`KismetSystemLibrary.DrawDebugSphere` (+ (`SceneComponent.K2_GetComponentLocation` (`self.DefaultSceneRoot`)) _returnvalue) 100.0 4 (struct :`R` 1.0 :`B` 0.220286 :`A` 1.0) 0.1 1.0)
    (`KismetArrayLibrary.Array_Add` (`local.NewLocalVar_1`) _returnvalue))
  (set `self.NewVar_0` (`local.NewLocalVar_1`)))