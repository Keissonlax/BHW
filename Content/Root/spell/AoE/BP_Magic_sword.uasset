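; BP_Magic_sword is an AoE spell actor that swings in a yaw arc around the player over its lifetime.
; It records its starting yaw on BeginPlay, then each tick feeds normalized timer progress through a float curve to interpolate a yaw offset from that heading.
; The root also snaps to player pawn 0's location every tick, so the swing follows the player.
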(event `self.ReceiveBeginPlay`
  (bind (_returnvalue_roll _returnvalue_pitch _returnvalue_yaw) (`KismetMathLibrary.BreakRotator` (`SceneComponent.K2_GetComponentRotation` (`self.DefaultSceneRoot`))))
  (`parent.ReceiveBeginPlay`)
  (set `self.Return Value Z (Yaw)` _returnvalue_yaw))

(event `self.ReceiveTick`
  (params (DeltaSeconds :type "Float (single-precision)"))
  (`parent.ReceiveTick` DeltaSeconds)
  (`SceneComponent.K2_SetWorldRotation` (`self.DefaultSceneRoot`) (`KismetMathLibrary.MakeRotator` 0.0 0.0 (+ (`KismetMathLibrary.Lerp` -100.0 90.0 (`CurveFloat.GetFloatValue` (`self.NewVar_0`) (/ (`KismetSystemLibrary.K2_GetTimerElapsedTimeHandle` (`self.Timer`)) (`self.LifeTime`)))) (`self.Return Value Z (Yaw)`))) false false)
  (`SceneComponent.K2_SetWorldLocation` (`self.DefaultSceneRoot`) (`self.K2_GetActorLocation` (`GameplayStatics.GetPlayerPawn` 0)) false false))

(fn `UserConstructionScript`
  (`parent.UserConstructionScript`))