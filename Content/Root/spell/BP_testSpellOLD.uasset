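; Test spell projectile, named as an old version, that flies in a wavy path and destroys itself after LifeTime.
; Start_Spell orients it along the given direction, starts the death timer and plays a Timeline.
; Each update steps it forward a fixed, non-delta-scaled distance plus a sideways cosine offset from timer elapsed time, Chastota (frequency) and Amplituda.
; Ground-trace and debug nodes are disconnected.
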(event `self.ReceiveTick`
  (params (DeltaSeconds :type "Float (single-precision)")))

(event `self.ReceiveBeginPlay`)

(event `dead`
  (`self.K2_DestroyActor`))

(event `Start_Spell`
  (params (direkion :type "Vector Structure"))
  (bind _defaultsceneroot (`self.DefaultSceneRoot`))
  (bind (_returnvalue_x _returnvalue_y _returnvalue_z) (`KismetMathLibrary.BreakVector` (`SceneComponent.GetForwardVector` _defaultsceneroot)))
  (bind _returnvalue (`KismetSystemLibrary.K2_SetTimerDelegate` (delegate `dead`) (`self.LifeTime`)))
  (set `self.Timer` _returnvalue)
  (bind _output_get (set `self.Direkion` direkion))
  (`SceneComponent.K2_SetWorldRotation` (`self.DefaultSceneRoot`) (`KismetMathLibrary.Conv_VectorToRotator` _output_get) false false)
  (`Timeline|Timeline`
    (:`Update`
      (`SceneComponent.K2_SetWorldLocation` _defaultsceneroot (+ (* (`KismetMathLibrary.MakeVector` _returnvalue_x _returnvalue_y _returnvalue_z) 15.0) (`self.K2_GetActorLocation`) (* (`KismetMathLibrary.RotateAngleAxis` _output_get 90.0 (0.0 0.0 1.0)) (* (`KismetMathLibrary.Cos` (* (`KismetSystemLibrary.K2_GetTimerElapsedTimeHandle` (`self.Timer`)) (`self.chastota`))) (`self.amplituda`)))) false false))))

(event `/Game/Root/spell/BPI_spellCast.CastSpell`)

(fn `UserConstructionScript`)