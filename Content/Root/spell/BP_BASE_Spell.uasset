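; Base spell actor that configures itself from the player character's current spell and destroys itself when its lifetime ends.
; On BeginPlay it reads the matching DT_Spell row for damage, lifetime and scale, derives a facing rotation, and starts the destroy timer.
; Tick delegates movement to attached Mod_Base components and prints timer debug text.
; Cast/start events are empty; mesh creation and mod initialization are disconnected.
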(event `self.CastSpell`)

(event `self.ReceiveTick`
  (params (DeltaSeconds :type "Float (single-precision)"))
  (`|ExecutionSequence`
    (:`then_0`
      (for _array_element (`self.K2_GetComponentsByClass` "/Game/Root/MOD/mod_Base.mod_Base_C")
        (`/Engine/EditorBlueprintResources/StandardMacros.IsValid` _array_element
          (:`Is Valid`
            (`/Game/Root/MOD/mod_Base.Move` _array_element 1.0)))))
    (:`then_1`
      (`KismetSystemLibrary.PrintString` (`KismetStringLibrary.Conv_DoubleToString` (`KismetSystemLibrary.K2_GetTimerElapsedTimeHandle` (stale `self.ReceiveBeginPlay` _output_get_2))) true true (struct :`R` 0.703612 :`G` 1.0 :`A` 1.0) 0.001))))

(event `self.ReceiveBeginPlay`
  (bind _asbp_my_char (cast `/Game/Root/Char/BP_MyChar` (`GameplayStatics.GetPlayerPawn` 0)))
  (set `self.As BP My Char` _asbp_my_char)
  (set `self.RowSpellName` (`/Game/Root/Char/BP_MyChar.CurentSpellName` _asbp_my_char))
  (`|ExecutionSequence`
    (:`then_0`
      (bind _returnvalue (`|GetDataTableRow` "/Game/Root/spell/DT_Spell.DT_Spell" (`self.RowSpellName`))
        (:`then`
          (`|ExecutionSequence`
            (:`then_0`
              (bind ((`ID_70_3B21157149B0957107735487C74C62A1` _id) (`Type_61_539C5CCE496AF32AC3896582DC6D72A1` _type) (`scale_36_8E0C3AE34DE2720FB969ECB1E17BFAE7` _scale) (`life_time_5_DBD29C6344A9156AAE7367ADBB2FED7B` _life_time) (`damage_8_E793A34346C3C7AC4A1556AF645BC39D` _damage) (`static_mesh_11_AA06FBFE4DDF35B9D4293EA7CEE24FF5` _static_mesh)) (break `/Game/Root/spell/S_Spell` _returnvalue))
              (set `self.Damage` _damage)
              (set `self.LifeTime` _life_time)
              (`|ExecutionSequence`
                (:`then_0`
                  (`SceneComponent.SetWorldScale3D` (`self.DefaultSceneRoot`) _scale)
                  (`|ExecutionSequence`
                    (:`then_1`
                      (bind _direction (`/Game/Root/MyFunctionLibrary.Char_vectors`))
                      (bind _output_get (set `self.Direction` _direction))
                      (set `self.CharRotation` (`KismetMathLibrary.Conv_VectorToRotator` _output_get))
                      (`|ExecutionSequence`
                        (:`then_0`
                          (bind _returnvalue_2 (`KismetSystemLibrary.K2_SetTimerDelegate` (delegate `dead`) (`self.LifeTime`)))
                          (bind _output_get_2 (set `self.Timer` _returnvalue_2)))))))))))))))

(event `dead`
  (`self.K2_DestroyActor`))

(event `Start_Spell`)

(fn `AplyMod`
  (for _array_element (`self.K2_GetComponentsByClass` "/Game/Root/MOD/mod_Base.mod_Base_C")
    (`/Game/Root/MOD/mod_Base.InitMod` _array_element null)))

(fn `UserConstructionScript`)