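; Magic barrier spell actor, filed under buff spells, that stays attached to the player by updating its transform manually.
; Every Tick it sets the root's world yaw from the character's MYRotation and moves the root to player pawn 0's location, without sweep.
; BeginPlay and Tick call the parent class first, and no barrier effect logic appears in these graphs.
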(event `self.ReceiveBeginPlay`
  (`parent.ReceiveBeginPlay`))

(event `self.ReceiveTick`
  (params (DeltaSeconds :type "Float (single-precision)"))
  (`parent.ReceiveTick` DeltaSeconds)
  (`SceneComponent.K2_SetWorldRotation` (`self.DefaultSceneRoot`) (`KismetMathLibrary.MakeRotator` 0.0 0.0 (`/Game/Root/Char/BP_MyChar.MY_Rotation` (`self.As BP My Char`))) false false)
  (`SceneComponent.K2_SetWorldLocation` (`self.DefaultSceneRoot`) (`self.K2_GetActorLocation` (`GameplayStatics.GetPlayerPawn` 0)) false false))

(fn `UserConstructionScript`
  (`parent.UserConstructionScript`))