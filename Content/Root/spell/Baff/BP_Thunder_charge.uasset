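; BP_Thunder_charge is a thunder-charge spell buff actor that follows the player pawn and emits brief periodic pulses.
; Each Tick moves its root to the player and shows Sphere1 only near the peaks of a sine wave over Timer's elapsed time.
; A DoOnce adds one enlarged sphere component per pulse, then destroys it and resets when the pulse ends.
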(event `self.ReceiveBeginPlay`
  (`parent.ReceiveBeginPlay`))

(event `self.ReceiveTick`
  (params (DeltaSeconds :type "Float (single-precision)"))
  (bind _newvar_0 (`self.NewVar_0`))
  (bind _returnvalue (> (`KismetMathLibrary.Sin` (* (`KismetSystemLibrary.K2_GetTimerElapsedTimeHandle` (`self.Timer`)) 10.0)) 0.95))
  (`parent.ReceiveTick` DeltaSeconds)
  (`SceneComponent.K2_SetWorldLocation` (`self.DefaultSceneRoot`) (`self.K2_GetActorLocation` (`GameplayStatics.GetPlayerPawn` 0)) false false)
  (`SceneComponent.SetVisibility` (`self.Sphere1`) _returnvalue false)
  (if _returnvalue
    (`/Engine/EditorBlueprintResources/StandardMacros.DoOnce` false :!label _label
      (:`Completed`
        (bind _returnvalue_2 (`AddComponent|NODE_AddSphereComponent-1` :`RelativeTransform` (`KismetMathLibrary.MakeTransform` (0.0 0.0 0.0) (struct) (10.0 10.0 10.0))))
        (set `self.NewVar_0` _returnvalue_2)))
    (else
      (`/Engine/EditorBlueprintResources/StandardMacros.IsValid` _newvar_0
        (:`Is Valid`
          (`ActorComponent.K2_DestroyComponent` _newvar_0)
          (goto _label :!via `Reset`))))))

(fn `UserConstructionScript`
  (`parent.UserConstructionScript`))