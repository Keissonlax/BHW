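; Base spell projectile actor that builds its look from a data table and destroys itself after a set lifetime.
; BeginPlay reads the hardcoded "spell1" row of DT_projectile for lifetime, mesh and scale, then adds a shadowless, collision-free static mesh component.
; Start_Spell starts a timer that calls dead to destroy the actor; its direction input is unused.
; CastSpell is an empty event, and the graph has no movement or hit logic.
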(event `dead`
  (`self.K2_DestroyActor`))

(event `Start_Spell`
  (params (direkion :type "Vector Structure"))
  (`|ExecutionSequence`
    (:`then_0`
      (bind _returnvalue (`KismetSystemLibrary.K2_SetTimerDelegate` (delegate `dead`) (`self.LifeTime`)))
      (set `self.Timer` _returnvalue))))

(event `self.CastSpell`)

(event `self.ReceiveTick`
  (params (DeltaSeconds :type "Float (single-precision)")))

(event `self.ReceiveBeginPlay`
  (bind _returnvalue (`|GetDataTableRow` "/Game/Root/spell/projectile/DT_projectile.DT_projectile" "spell1")
    (:`then`
      (bind (_name _description _scale _position _base_speed _life_time _damage _magic_type_damage _static_mesh) (break `/Game/Root/spell/projectile/S_SpellProjectileBase` _returnvalue))
      (set `self.LifeTime` _life_time)
      (bind _returnvalue_2 (`AddComponent|NODE_AddStaticMeshComponent-0`))
      (`PrimitiveComponent.SetCollisionEnabled` _returnvalue_2 "NoCollision")
      (`SceneComponent.SetRelativeScale3D` _returnvalue_2 _scale)
      (`PrimitiveComponent.SetCastShadow` _returnvalue_2 false)
      (`StaticMeshComponent.SetStaticMesh` _returnvalue_2 _static_mesh))))

(fn `UserConstructionScript`)