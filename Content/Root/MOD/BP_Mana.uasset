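; BP_Mana is a small Blueprint that adds a flat bonus to the Mana of the character referenced by BPChar at BeginPlay.
; After calling the parent and waiting briefly, it prints a debug string based on whether BPChar is valid.
; Both branches then reach the Mana increase, so it runs even when the reference is invalid.
; Nothing here assigns BPChar, and Tick is disabled.
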(event `self.ReceiveBeginPlay`
  (bind _bp_char (`self.BP_Char`))
  (`parent.ReceiveBeginPlay`)
  (`KismetSystemLibrary.Delay` 0.2)
  (`/Engine/EditorBlueprintResources/StandardMacros.IsValid` _bp_char
    (:`Is Valid`
      (`KismetSystemLibrary.PrintString` "Hello"))
    (:`Is Not Valid`
      (`KismetSystemLibrary.PrintString` "YTN")))
  (set `/Game/Root/Char/BP_MyChar.Mana` (+ (`/Game/Root/Char/BP_MyChar.Mana` _bp_char) 5.0) _bp_char))