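; BP_Trio appears to be a spell modifier that multiplies the spell in TestSpellRef by spawning extra copies of it.
; Shortly after BeginPlay, a two-pass loop spawns the same class at the spell's location, stepping an accumulated yaw offset by 30 degrees to fan the copies.
; Logic to copy BPAC_BASE_mod components onto spawned spells is unconnected, and a debug "Hello" prints on each pass.
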(event `self.ReceiveBeginPlay`
  (bind _test_spell_ref (`self.test_spell_ref`))
  (bind (_returnvalue_roll _returnvalue_pitch _returnvalue_yaw) (`KismetMathLibrary.BreakRotator` (`Actor.K2_GetActorRotation` (`self.test_spell_ref`))))
  (`parent.ReceiveBeginPlay`)
  (`KismetSystemLibrary.Delay` 0.001)
  (for _ (range 2)
    (`KismetSystemLibrary.PrintString` "Hello")
    (bind _returnvalue (`|SpawnActorFromClass` (`GameplayStatics.GetObjectClass` _test_spell_ref) (`KismetMathLibrary.MakeTransform` (`Actor.K2_GetActorLocation` _test_spell_ref) (`KismetMathLibrary.MakeRotator` _returnvalue_roll _returnvalue_pitch (+ _returnvalue_yaw (`self.Spawn Transform Rotation Z (Yaw)`)))) "Undefined" "MultiplyWithRoot" null "spell1" false null))
    (set `self.Spawn Transform Rotation Z (Yaw)` (+ (`self.Spawn Transform Rotation Z (Yaw)`) 30.0))))