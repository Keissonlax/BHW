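; BP_ModMove is a spell modifier that moves its owning BP_BASE_Spell forward.
; Its Move function casts the owner and offsets the spell's root component along its forward vector by the current spell's BaseSpeed times the DopSped multiplier.
; Each call sets world location directly without sweep or delta-time scaling, and the asset's own BeginPlay and Tick are disabled.
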(fn `Move`
  (params (DopSped :type "Float (double-precision)" :default 0.0))
  (bind _asbp_base_spell (cast `/Game/Root/spell/BP_BASE_Spell` (`self.GetOwner`)))
  (set `self.Root Component` (`Actor.RootComponent` _asbp_base_spell))
  (`SceneComponent.K2_SetWorldLocation` (`self.Root Component`) (+ (* (`SceneComponent.GetForwardVector` (`self.Root Component`)) (* (`.base_speed_21_6350F2074F0B68B1DCEA35B4E608B014` (break `/Game/Root/spell/S_Spell` (`/Game/Root/spell/BP_BASE_Spell.Current Spell` _asbp_base_spell))) (`local.DopSped`))) (`SceneComponent.K2_GetComponentLocation` (`self.Root Component`))) false false))