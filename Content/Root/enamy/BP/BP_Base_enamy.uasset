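; Base enemy Blueprint that takes damage from spells and can drop a magic gem on death.
; BeginPlay loads stats from DT_Enamy_Data by row name and sets up an HP widget, which Tick turns toward the player camera.
; Overlapping spells subtract raw damage, calling an empty Dmg event or, at zero HP, randomly spawning a gem picked through the player's inventory before destruction.
; Attack sphere-traces ahead and returns whether it hit the player.
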(event `self.ReceiveBeginPlay`
  (bind _asbp_my_char (cast `/Game/Root/Char/BP_MyChar` (`GameplayStatics.GetPlayerPawn` 0)))
  (set `self.As BP My Char` _asbp_my_char)
  (bind _returnvalue (`|GetDataTableRow` "/Game/Root/enamy/DT_Enamy_Data.DT_Enamy_Data" (`self.Row Name`))
    (:`then`
      (bind (_name _hp _attack _walkspeed _physdeffens _magdeffens _physinvulnerability) (break `/Game/Root/enamy/S_Enamy_Data` _returnvalue))
      (bind _output_get (set `self.HP` _hp))
      (set `self.Damage` _attack)
      (set `self.Walk speed` _walkspeed)
      (set `self.Phys Deffens` _physdeffens)
      (set `self.Mag Deffens` _magdeffens)
      (set `self.Phys Invulnerability` _physinvulnerability)
      (set `self.HP_Max` _output_get)
      (bind _aswb_enamy_hp (cast `/Game/Root/enamy/WB_enamyHP` (`WidgetComponent.GetWidget` (`self.Widget`))))
      (`/Game/Root/enamy/WB_enamyHP.Setap` _aswb_enamy_hp self))))

(event `self.ReceiveActorBeginOverlap`
  (params (OtherActor :type "Actor Object Reference"))
  (bind _asbp_base_spell (cast `/Game/Root/spell/BP_BASE_Spell` OtherActor))
  (set `self.HP` (- (`self.HP`) (`/Game/Root/spell/BP_BASE_Spell.Damage` _asbp_base_spell)))
  (if (<= (`self.HP`) 0)
    (`self.Drop_loot` 0.5)
    (`self.K2_DestroyActor`)
    (else
      (`self.Dmg`)
      (`KismetSystemLibrary.PrintString` (`KismetStringLibrary.Conv_IntToString` (`self.HP`))))))

(event `Dmg`)

(event `self.ReceiveTick`
  (params (DeltaSeconds :type "Float (single-precision)"))
  (bind _asbp_my_char (cast `/Game/Root/Char/BP_MyChar` (`GameplayStatics.GetPlayerPawn` 0)))
  (`SceneComponent.K2_SetWorldRotation` (`self.Widget`) (`KismetMathLibrary.RInterpTo` (`SceneComponent.K2_GetComponentRotation` (`self.Widget`)) (`KismetMathLibrary.FindLookAtRotation` (`SceneComponent.K2_GetComponentLocation` (`self.CapsuleComponent`)) (`SceneComponent.K2_GetComponentLocation` (`/Game/Root/Char/BP_MyChar.MyCamera` _asbp_my_char))) 0.01 5.0) false false))

(fn `Attack`
  (returns (NewParam :type Boolean))
  (bind _returnvalue (+ (`SceneComponent.K2_GetComponentLocation` (`self.Mesh`)) (* (`KismetMathLibrary.Normal` (`self.GetActorForwardVector`)) 200.0)))
  (bind _outhit (`KismetSystemLibrary.SphereTraceSingleForObjects` :`Start` _returnvalue :`End` _returnvalue :`Radius` 200.0 :`ObjectTypes` (`|MakeArray` "ObjectTypeQuery3" :!type "EObjectTypeQuery Enum") :`DrawDebugType` "ForDuration" :`DrawTime` 3.5))
  (cast `/Game/Root/Char/BP_MyChar` (`.HitActor` (`GameplayStatics.BreakHitResult` _outhit))
    (:`then`
      (`KismetSystemLibrary.PrintString` "ИГРОК" true true (struct :`R` 0.134131 :`G` 1.0 :`A` 1.0))
      (return true))
    (:`CastFailed`
      (`KismetSystemLibrary.PrintString` "НЕ ИГРОК" true true (struct :`R` 0.134131 :`G` 1.0 :`A` 1.0))
      (return false))))

(fn `Drop_loot`
  (params (B :type "Float (double-precision)"))
  (locals (NewLocalVar :type Name))
  (bind (_returnvalue_x _returnvalue_y _returnvalue_z) (`KismetMathLibrary.BreakVector` (`SceneComponent.K2_GetComponentLocation` (`Actor.RootComponent` (`self.As BP My Char`)))))
  (bind (_returnvalue_x_2 _returnvalue_y_2) (`KismetMathLibrary.BreakVector` (+ (`SceneComponent.K2_GetComponentLocation` (`self.CapsuleComponent`)) (0.0 0.0 100.0))))
  (if (> (`KismetMathLibrary.RandomFloatInRange` 0.0 1.0) B)
    (set `local.NewLocalVar` (`KismetArrayLibrary.Array_Random` (`/Game/Root/spell/Inventory/BPAC_New_Inventory.Test` (`/Game/Root/Char/BP_MyChar.BPAC_New_Inventory` (`self.As BP My Char`)))))
    (bind _returnvalue (`|GetDataTableRow` "/Game/Root/spell/DT_Spell.DT_Spell" (`local.NewLocalVar`))
      (:`then`
        (`|SpawnActorFromClass` "/Game/Root/spell/SpellGem/BP_New_Magic_Gem.BP_New_Magic_Gem_C" (`KismetMathLibrary.MakeTransform` (`KismetMathLibrary.MakeVector` _returnvalue_x_2 _returnvalue_y_2 _returnvalue_z)) "Undefined" "MultiplyWithRoot" null _returnvalue (`local.NewLocalVar`) null)))))

(fn `UserConstructionScript`)