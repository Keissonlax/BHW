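; BP_Golem is a golem enemy Blueprint with an attack hit check and a component cleanup function.
; Attack runs a zero-length sphere trace for Pawns ahead of the Test component, with debug drawing.
; It returns whether the hit actor is BP_MyChar and prints a Russian player/not-player message.
; Destroy removes the NewVar component; the event graph and construction script are empty.
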(event `self.ReceiveBeginPlay`)

(fn `Attack`
  (returns (NewParam :type Boolean))
  (bind _returnvalue (+ (`SceneComponent.K2_GetComponentLocation` (`self.test`)) (* (`KismetMathLibrary.Normal` (`self.GetActorForwardVector`)) 200.0)))
  (bind _outhit (`KismetSystemLibrary.SphereTraceSingleForObjects` :`Start` _returnvalue :`End` _returnvalue :`Radius` 200.0 :`ObjectTypes` (`|MakeArray` "ObjectTypeQuery3" :!type "EObjectTypeQuery Enum") :`DrawDebugType` "ForDuration" :`DrawTime` 3.5))
  (cast `/Game/Root/Char/BP_MyChar` (`.HitActor` (`GameplayStatics.BreakHitResult` _outhit))
    (:`then`
      (`KismetSystemLibrary.PrintString` "ИГРОК" true true (struct :`R` 0.134131 :`G` 1.0 :`A` 1.0))
      (return true))
    (:`CastFailed`
      (`KismetSystemLibrary.PrintString` "НЕ ИГРОК" true true (struct :`R` 0.134131 :`G` 1.0 :`A` 1.0))
      (return false))))

(fn `destroy`
  (`ActorComponent.K2_DestroyComponent` (`self.NewVar`))
  (return))

(fn `UserConstructionScript`)