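; BP_test_enamy is a test enemy actor that takes spell damage and is destroyed when its HP runs out.
; Sphere overlaps with a BP_BASE_Spell subtract that spell's Damage from HP, which starts at MaxHP.
; A hit handler feeds the HP ratio to the WB_enamyHP widget's progress bar.
; Tick turns the widget toward the player's camera and prints HP for debugging.
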(event `self.ReceiveBeginPlay`
  (set `self.HP` (`self.MaxHP`)))

(event `self.ReceiveTick`
  (params (DeltaSeconds :type "Float (single-precision)"))
  (`KismetSystemLibrary.PrintString` (`KismetStringLibrary.Conv_IntToString` (`self.HP`)) true true (struct :`R` 1.0 :`G` 0.161295 :`A` 1.0) 0.001)
  (bind _asbp_my_char (cast `/Game/Root/Char/BP_MyChar` (`GameplayStatics.GetPlayerPawn` 0)))
  (`SceneComponent.K2_SetWorldRotation` (`self.Widget`) (`KismetMathLibrary.FindLookAtRotation` (`SceneComponent.K2_GetComponentLocation` (`self.DefaultSceneRoot`)) (`SceneComponent.K2_GetComponentLocation` (`/Game/Root/Char/BP_MyChar.MyCamera` _asbp_my_char))) false false))

(event `self.Sphere.OnComponentBeginOverlap`
  (params (OverlappedComponent :type "PrimitiveComponent Object Reference") (OtherActor :type "Actor Object Reference") (OtherComp :type "PrimitiveComponent Object Reference") (OtherBodyIndex :type Integer) (bFromSweep :type Boolean) (SweepResult :type "HitResult Structure (by ref)"))
  (`/Engine/EditorBlueprintResources/StandardMacros.IsValid` OtherActor
    (:`Is Valid`
      (bind _asbp_base_spell (cast `/Game/Root/spell/BP_BASE_Spell` OtherActor))
      (bind _damage (`/Game/Root/spell/BP_BASE_Spell.Damage` _asbp_base_spell))
      (`KismetSystemLibrary.PrintString` (`KismetStringLibrary.Conv_IntToString` _damage))
      (set `self.HP` (- (`self.HP`) _damage))
      (`|ExecutionSequence`
        (:`then_0`
          (if (<= (`self.HP`) 0)
            (`self.K2_DestroyActor`)))
        (:`then_1`
          (`self.Get_dmg`)
          (`KismetSystemLibrary.PrintString` "удар"))))))

(event `Get_dmg`
  (bind _widget (`self.Widget`))
  (bind _returnvalue (/ (`KismetMathLibrary.Conv_IntToDouble` (`self.HP`)) (`KismetMathLibrary.Conv_IntToDouble` (`self.MaxHP`))))
  (`/Engine/EditorBlueprintResources/StandardMacros.IsValid` _widget
    (:`Is Valid`
      (bind _aswb_enamy_hp (cast `/Game/Root/enamy/WB_enamyHP` (`WidgetComponent.GetWidget` _widget)))
      (`KismetSystemLibrary.PrintString` (`KismetStringLibrary.Conv_DoubleToString` _returnvalue))
      (`ProgressBar.SetPercent` (`/Game/Root/enamy/WB_enamyHP.ProgressBar_118` _aswb_enamy_hp) _returnvalue))))

(fn `UserConstructionScript`)